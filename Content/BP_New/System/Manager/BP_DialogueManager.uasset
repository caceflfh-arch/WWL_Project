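; Dialogue manager actor that runs data-table-driven NPC conversations through WB_Dialogue.
; PlayNext finds rows by sequence and index, filters reactions by grade, shows text or choices, and follows NextSq links.
; Event rows trigger NPC animations, spawned timeline cinematics or level sequences, while BP_EventManager gates advancement on wait events.
; Choices track used IDs and can return to hubs; finished sequences trigger hardcoded follow-ups such as spawning a test NPC.
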(event `self.ReceiveBeginPlay`
  (bind _returnvalue (`GameplayStatics.GetActorOfClass` "/Game/BP_New/System/Manager/BP_EventManager.BP_EventManager_C"))
  (set `self.EventManagerRef` _returnvalue))

(event `PlayLevelSequence`
  (params (LevelSequenceRef :type "LevelSequence Object Reference"))
  ;[1 1 1] sequence play (with duration)
  (bind (_outactor _returnvalue) (`LevelSequencePlayer.CreateLevelSequencePlayer` LevelSequenceRef))
  (`MovieSceneSequencePlayer.Play` _returnvalue)
  (`KismetSystemLibrary.Delay` (`TimeManagementBlueprintLibrary.Conv_QualifiedFrameTimeToSeconds` (`MovieSceneSequencePlayer.GetDuration` _returnvalue)))
  (set `self.bIsEventRunning` false)
  (`self.TryAdvanceDialogue`)
  (`UserWidget.AddToViewport` (`self.DialogueWidget`) 0)
  (`self.PlayNext`))

(event `StartDay1SQ102`
  (`self.StartDialogue` 102 null "NewEnumerator4" "/Game/BP_New/Data/DT_Day1.DT_Day1" 1))

(fn `CheckWaitingEvent`
  (bind _currentwaitevent (`self.CurrentWaitEvent`))
  (if (== _currentwaitevent "None")
    (return)
    (else
      (bind _bool (`/Game/BP_New/System/Manager/BP_EventManager.HasCompleted` (`self.EventManagerRef`) _currentwaitevent))
      (if _bool
        (`/Engine/EditorBlueprintResources/StandardMacros.IncrementInt` (`self.CurrentDialogueIndex`)
          (:`  `
            (`/Engine/EditorBlueprintResources/StandardMacros.IncrementInt` (`self.LoopCount`))))))))

(fn `ConfirmChoice`
  (bind _currentchoiceindex (`self.CurrentChoiceIndex`))
  (bind (_choiceid _choicetext _choicesq _notremoveafterchoice _resetlastchoiceindex) (break `/Game/BP_New/Data/FS_Choice` (`/Game/BP_New/UI/WB_ChoiceButton.ChoiceData` (`|GetArrayItem` (`self.ChoiceButtonArray`) _currentchoiceindex))))
  (set `self.LastChoiceIndex` _currentchoiceindex)
  (set `self.bIsWaitingForChoice` false)
  (if (not _notremoveafterchoice)
    (`KismetArrayLibrary.Array_Add` (`self.UsedChoiceIDs`) (`KismetStringLibrary.Conv_NameToString` _choiceid)))
  (if _resetlastchoiceindex
    (set `self.LastChoiceIndex` 0))
  ;[1 1 1] 컨테이너, 버튼 UI 초기화
  (`PanelWidget.ClearChildren` (`/Game/BP_New/UI/WB_Dialogue.ChoiceContainer` (`self.DialogueWidget`)))
  (set `self.CurrentSq` _choicesq)
  (`KismetArrayLibrary.Array_Clear` (`self.ChoiceButtonArray`))
  (set `self.CurrentDialogueIndex` 1)
  (`self.PlayNext`))

(fn `GetDialogueRow`
  (params (InSq :type Integer) (InIndex :type Integer))
  (returns (OutRow :type "/Game/BP_New/Data/FS_Dialogue Structure") (RowFound :type Boolean))
  (locals (Local_Found :type Boolean) (Local_Row :type "/Game/BP_New/Data/FS_Dialogue Structure"))
  (bind _currentdatatable (`self.CurrentDataTable`))
  (set `local.Local_Found` false)
  (bind _outrownames (`DataTableFunctionLibrary.GetDataTableRowNames` _currentdatatable))
  (for _array_element _outrownames
    (bind _returnvalue (`|GetDataTableRow` _currentdatatable _array_element)
      (:`then`
        (bind (_sqindex _dialogindex _nextsq _nodetype _eventdata _speakername _dialoguetext _playerchoice _choicearray _grade) (break `/Game/BP_New/Data/FS_Dialogue` _returnvalue))
        (if (and (and (== _sqindex InSq) (== _dialogindex InIndex)) (or (`|EnumInequality` _nodetype "NewEnumerator1") (`|EnumEquality` _grade (`self.CurrentGrade`))))
          (bind _output_get (set `local.Local_Row` _returnvalue))
          (set `local.Local_Found` true)
          (set `self.LastValidRow` _output_get)
          (break)))))
  (return (`local.Local_Row`) (`local.Local_Found`)))

(fn `HandleFlowFinished`
  (params (FinishedSQ :type Integer))
  (switch `int` (`self.CurrentDay`)
    (:`1`
      (switch `int` FinishedSQ
        (:`Default`
          (return))
        (:`101`
          (`KismetSystemLibrary.K2_SetTimerDelegate` (`|CreateDelegate` :!event `StartDay1SQ102`) 1.0))
        (:`102`
          ;[1 1 1] test
          (`|SpawnActorFromClass` "/Game/BP_New/Interaction/BP_NPC_Test.BP_NPC_Test_C" (`KismetMathLibrary.MakeTransform` (349.031769 244.890671 0.0) (struct :`Yaw` 140.0)) "Undefined" "MultiplyWithRoot" null null null))))))

(fn `PlayNext`
  (bind _dialoguewidget (`self.DialogueWidget`))
  (bind (_sqindex _dialogindex _nextsq _nodetype _eventdata _speakername _dialoguetext _playerchoice _choicearray _grade) (break `/Game/BP_New/Data/FS_Dialogue` (`self.CurrentRow`)))
  (bind (_sqindex_2 _dialogindex_2 _nextsq_2 _nodetype_2 _eventdata_2 _speakername_2 _dialoguetext_2 _playerchoice_2 _choicearray_2 _grade_2 _bhidedialogueui _waitforfinish) (break `/Game/BP_New/Data/FS_Dialogue` (`self.CurrentRow`)))
  (bind (_sqindex_3 _dialogindex_3 _nextsq_3 _nodetype_3 _eventdata_3 _speakername_3 _dialoguetext_3 _playerchoice_3 _choicearray_3 _grade_3 _bhidedialogueui_2 _waitforfinish_2 _lastdialogue _returntochoicehub _choicehubsq) (break `/Game/BP_New/Data/FS_Dialogue` (`self.CurrentRow`)))
  (bind (_sqindex_4 _dialogindex_4 _nextsq_4 _nodetype_4 _eventdata_4 _speakername_4 _dialoguetext_4 _playerchoice_4 _choicearray_4) (break `/Game/BP_New/Data/FS_Dialogue` (`self.LastValidRow`)))
  (bind (_eventtype _soundasset _timelineactor _animationtype _levelsequence) (break `/Game/BP_New/Data/FS_EventData` (`|GetArrayItem` _eventdata_2)))
  (if (`self.bIsEventRunning`)
    (`KismetSystemLibrary.PrintString` "event running")
    (else
      (bind (_outrow _rowfound) (`self.GetDialogueRow` (`self.CurrentSq`) (`self.CurrentDialogueIndex`)))
      (set `self.CurrentRow` _outrow)
      (set `self.Row_NextSq` _nextsq)
      (set `self.Row_NodeType` _nodetype)
      (set `self.Row_Text` _dialoguetext)
      (set `self.Row_Speaker` _speakername)
      (set `self.Row_Grade` _grade)
      (if _rowfound
        (if _playerchoice_4
          (set `self.bIsWaitingForChoice` true)
          (for _array_element _choicearray_4
            (bind _returnvalue (`|CreateWidget` "/Game/BP_New/UI/WB_ChoiceButton.WB_ChoiceButton_C"))
            (`KismetArrayLibrary.Array_Add` (`self.ChoiceButtonArray`) _returnvalue)
            (if (`KismetArrayLibrary.Array_Contains` (`self.UsedChoiceIDs`) (`KismetStringLibrary.Conv_NameToString` (`.ChoiceID_2_9DAB30DE41CCE35ECEACFA886BCACD82` (break `/Game/BP_New/Data/FS_Choice` _array_element))))
              (`/Game/BP_New/UI/WB_ChoiceButton.SetDisabled` _returnvalue true))
            (`/Game/BP_New/UI/WB_ChoiceButton.SetChoice` _returnvalue _array_element)
            (`VerticalBox.AddChildToVerticalBox` (`/Game/BP_New/UI/WB_Dialogue.ChoiceContainer` (`self.DialogueWidget`)) _returnvalue))
          (set `self.CurrentChoiceIndex` (`self.LastChoiceIndex`))
          (`self.UpdateChoiceVisual`)
          (else
            (switch `/Game/BP_New/Data/E_NodeType` (`self.Row_NodeType`)
              (:`NewEnumerator0`
                (`/Game/BP_New/UI/WB_Dialogue.SetDialogueText` (`self.DialogueWidget`) (`self.Row_Speaker`) (`self.Row_Text`))
                (`self.TryAdvanceDialogue` :!label _label))
              (:`NewEnumerator1`
                (`/Game/BP_New/UI/WB_Dialogue.SetDialogueText` (`self.DialogueWidget`) (`self.Row_Speaker`) (`self.Row_Text`))
                (goto _label))
              (:`NewEnumerator2`
                (set `self.bIsEventRunning` true)
                (if _bhidedialogueui
                  (`/Engine/EditorBlueprintResources/StandardMacros.IsValid` _dialoguewidget
                    (:`Is Valid`
                      (`Widget.RemoveFromParent` _dialoguewidget))
                    (:`Is Not Valid`
                      _))
                  (else
                    (`/Game/BP_New/UI/WB_Dialogue.SetDialogueText` (`self.DialogueWidget`) (`self.Row_Speaker`) (`self.Row_Text`))))
                (switch `/Game/BP_New/Data/E_EventType` _eventtype
                  (:`NewEnumerator0`
                    (`/Game/BP_New/Interaction/BP_NPC_Base.PlayAnimation` (`self.CurrentNPC`) _animationtype null self _bhidedialogueui _waitforfinish))
                  (:`NewEnumerator5`
                    (bind _returnvalue_2 (`|SpawnActorFromClass` _timelineactor (`KismetMathLibrary.MakeTransform` (0.0 0.0 0.0)) "Undefined" "MultiplyWithRoot" null null))
                    (bind _asbp_timeline_player (cast `/Game/BP_New/Timeline/BP_TimelinePlayer` _returnvalue_2))
                    (`/Game/BP_New/Timeline/BP_TimelinePlayer.PlayCinematic` _asbp_timeline_player self _bhidedialogueui))
                  (:`NewEnumerator6`
                    (`self.PlayLevelSequence` _levelsequence)))))
            (if _returntochoicehub
              (set `self.CurrentSq` _choicehubsq)
              (set `self.CurrentDialogueIndex` 1))))
        (elif (== _nextsq_4 0)
          (`KismetSystemLibrary.PrintString` "\"Dialogue 종료됨\"")
          (`Widget.RemoveFromParent` (`self.DialogueWidget`)) ; Dialogue 종료지점
          (set `self.bIsDialoguePlaying` false)
          (`self.HandleFlowFinished` _sqindex_4)
          (else
            (set `self.CurrentSq` _nextsq_4)
            (set `self.CurrentDialogueIndex` 1)
            (`self.PlayNext`)))))))

(fn `ReturnToPlayerCamera`)

(fn `StartDialogue`
  (params (StartSq :type Integer) (NPC :type "/Game/BP_New/Interaction/BP_NPC_Base Object Reference") (Grade :type "/Game/BP_New/Data/E_OverallGrade Enum" :default "NewEnumerator4") (SetDatatable :type "DataTable Object Reference") (CurrentDay :type Integer))
  (if (`self.bIsDialoguePlaying`)
    (return)
    (else
      (set `self.CurrentDataTable` SetDatatable)
      (set `self.CurrentDay` CurrentDay)
      (set `self.CurrentSq` StartSq)
      (set `self.CurrentDialogueIndex` 1)
      (set `self.CurrentNPC` NPC)
      (set `self.CurrentGrade` Grade)
      (set `self.bIsDialoguePlaying` true)
      (bind _returnvalue (`|CreateWidget` "/Game/BP_New/UI/WB_Dialogue.WB_Dialogue_C"))
      (bind _output_get (set `self.DialogueWidget` _returnvalue))
      (`UserWidget.AddToViewport` _output_get 0)
      (`self.PlayNext`))))

(fn `TryAdvanceDialogue`
  (bind (_triggerevent _waitevent) (break `/Game/BP_New/Data/FS_EventIDData` (`.EventID_87_A8B680DE4C35A5777AC663A992A08FD1` (break `/Game/BP_New/Data/FS_Dialogue` (`self.CurrentRow`)))))
  (if (== _waitevent "None")
    (`/Engine/EditorBlueprintResources/StandardMacros.IncrementInt` (`self.CurrentDialogueIndex`)
      (:`  `
        (`/Engine/EditorBlueprintResources/StandardMacros.IncrementInt` (`self.LoopCount`))))
    (else
      (set `self.CurrentWaitEvent` _waitevent)
      (`self.CheckWaitingEvent`))))

(fn `UpdateChoiceVisual`
  (for (_array_element _array_index) (`self.ChoiceButtonArray`)
    (if (== _array_index (`self.CurrentChoiceIndex`))
      (`/Game/BP_New/UI/WB_ChoiceButton.SetSelected` _array_element true)
      (else
        (`/Game/BP_New/UI/WB_ChoiceButton.SetSelected` _array_element false)))))

(fn `UserConstructionScript`)