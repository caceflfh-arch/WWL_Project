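; BP_EventManager is a manager that records which game events have completed.
; CompleteEvent adds each EventID to CompletedEvents once and prints a debug message, while HasCompleted queries that collection and ClearEvent is an empty stub.
; A legacy old_StartSequence stores a grade, issues back-to-back camera fades and starts a dialogue sequence, with a disconnected test NPC spawn left beside it.
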(event `self.ReceiveBeginPlay`)

(fn `ClearEvent`)

(fn `CompleteEvent`
  (params (EventID :type Name))
  (if (`BlueprintSetLibrary.Set_Contains` (`self.CompletedEvents`) EventID)
    (return)
    (else
      (`BlueprintSetLibrary.Set_Add` (`self.CompletedEvents`) EventID)
      (`KismetSystemLibrary.PrintString` (`KismetStringLibrary.Concat_StrStr` "[Event] Completed : " (`KismetStringLibrary.Conv_NameToString` EventID))))))

(fn `HasCompleted`
  (params (EventID :type Name))
  (returns (Bool :type Boolean))
  (return (`BlueprintSetLibrary.Set_Contains` (`self.CompletedEvents`) EventID)))

(fn `old_StartSequence`
  (params (Grade :type "/Game/BP_New/Data/E_OverallGrade Enum" :default "NewEnumerator4"))
  (bind _playercameramanager (`PlayerController.PlayerCameraManager` (`GameplayStatics.GetPlayerController` 0)))
  (set `self.old_StoredGrade` Grade)
  (`PlayerCameraManager.StartCameraFade` :`self` _playercameramanager :`ToAlpha` 1.0 :`Duration` 1.0)
  (`PlayerCameraManager.StartCameraFade` :`self` _playercameramanager :`FromAlpha` 1.0 :`Duration` 1.0)
  (`/Game/BP_New/System/Manager/BP_DialogueManager.StartDialogue` (`self.old_DialogueManagerRef`) 101 null "NewEnumerator4" null 0))

(fn `UserConstructionScript`)