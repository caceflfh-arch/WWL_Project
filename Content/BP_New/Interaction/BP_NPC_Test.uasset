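; Test NPC child Blueprint that plugs into the dialogue system for interaction.
; StartDialogue finds the first BP_DialogueManager in the level and starts a fixed sequence from DT_Day1, passing itself as the NPC and a hard-coded grade.
; PlayAnimation overrides the parent to map the Test Gesture type to a hand gesture montage before handing playback to the parent.
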(event `/Game/BP_New/Workobject/BPI_NPC.StartDialogue`
  (bind _outactors (`GameplayStatics.GetAllActorsOfClass` "/Game/BP_New/System/Manager/BP_DialogueManager.BP_DialogueManager_C"))
  (`/Game/BP_New/System/Manager/BP_DialogueManager.StartDialogue` (`|GetArrayItem` _outactors) 103 self "NewEnumerator0" "/Game/BP_New/Data/DT_Day1.DT_Day1" 0))

(fn `old_ShowNextDialogue`
  (params (DataTable :type "DataTable Object Reference"))
  (`parent.old_ShowNextDialogue` "/Game/BP_New/Data/none_DT_NPCReaction.none_DT_NPCReaction"))

(fn `PlayAnimation`
  (params (AnimationType :type "/Game/BP_New/Data/E_AnimationType Enum" :default "NewEnumerator2") (MontageRef :type "AnimMontage Object Reference") (DialogueManager :type "/Game/BP_New/System/Manager/BP_DialogueManager Object Reference") (PauseDialogue :type Boolean) (WaitForFinish :type Boolean))
  (switch `/Game/BP_New/Data/E_AnimationType` AnimationType
    (:`NewEnumerator1`
      (bind _output_get (set `self.MontageRef` "/Game/Character/TestNPC/HandGesture_Montage.HandGesture_Montage"))
      (`parent.PlayAnimation` "NewEnumerator0" _output_get DialogueManager PauseDialogue WaitForFinish))))

(fn `UserConstructionScript`
  (`parent.UserConstructionScript`))