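; Base NPC Blueprint for interaction: it cannot be picked up and plays animation montages as events within dialogue.
; PlayAnimation either lets the dialogue manager advance immediately or binds montage end to ResumeDialogue and PlayNext, re-showing the widget if dialogue was paused.
; StartDialogue and ShowDialogue are empty events.
; The old_ functions hold an earlier widget dialogue flow reading DT_HaenainHut_Dialogue by sequence and line index.
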(event `ShowDialogue`)

(event `/Game/BP_New/Workobject/BPI_NPC.StartDialogue`)

(event `OnMontageEnded`
  (params (Montage :type "AnimMontage Object Reference") (bInterrupted :type Boolean))
  (`self.ResumeDialogue`)
  (`/Game/BP_New/System/Manager/BP_DialogueManager.PlayNext` (`self.DialogueManagerRef`)))

(fn `CanPickup`
  (returns (ReturnValue :type Boolean))
  (return false))

(fn `old_EndDialogue`
  (bind _returnvalue (`GameplayStatics.GetPlayerController` 0))
  (`Widget.RemoveFromParent` (`self.DialogueWidget`))
  (`WidgetBlueprintLibrary.SetInputMode_GameOnly` _returnvalue)
  (set `PlayerController.bShowMouseCursor` false _returnvalue)
  (set `self.DialogueWidget` null))

(fn `old_ShowNextDialogue`
  (params (DataTable :type "DataTable Object Reference"))
  (if (== (`self.bIsInteracting`) false)
    (`/Engine/EditorBlueprintResources/StandardMacros.IsValid` (`self.DialogueWidget`)
      (:`Is Valid`
        (bind _output_get (set `self.CurrentDialogue` (`self.CurrentDialogue`)))
        (`/Engine/EditorBlueprintResources/StandardMacros.IncrementInt` _output_get
          (:`  `
            (bind _outrownames (`DataTableFunctionLibrary.GetDataTableRowNames` "/Game/BP_New/Data/DT_HaenainHut_Dialogue.DT_HaenainHut_Dialogue"))
            (for _array_element _outrownames
              (bind _returnvalue (`|GetDataTableRow` "/Game/BP_New/Data/DT_HaenainHut_Dialogue.DT_HaenainHut_Dialogue" _array_element)
                (:`then`
                  (bind _output_get_2 (set `self.TempRow` _returnvalue))
                  (bind (_sqindex _dialogindex _nextsq _nodetype _eventdata _speakername _dialoguetext _playerchoice _choicearray _grade _bhidedialogueui _waitforfinish _lastdialogue) (break `/Game/BP_New/Data/FS_Dialogue` _output_get_2))
                  (if (`KismetMathLibrary.Conv_IntToBool` (`KismetMathLibrary.And_IntInt` (`KismetMathLibrary.Conv_BoolToInt` (== (`self.CurrentSq`) _sqindex)) (`KismetMathLibrary.Conv_BoolToInt` (== _dialogindex (`self.CurrentDialogue`)))))
                    (`TextBlock.SetText` (`/Game/BP_New/UI/WB_Dialogue.TB_Dialogue` (`self.DialogueWidget`)) _dialoguetext)
                    (if (== _lastdialogue true)
                      (`self.old_EndDialogue`)
                      (return)
                      (else
                        (for _ _ :!via `Break`
                          _))))))))))
      (:`Is Not Valid`
        (return)))))

(fn `old_StartDialogue_Main`
  (`|ExecutionSequence`
    (:`then_0`
      (bind _returnvalue (`|CreateWidget` "/Game/BP_New/UI/WB_Dialogue.WB_Dialogue_C" (`GameplayStatics.GetPlayerController` 0)))
      (bind _output_get (set `self.DialogueWidget` _returnvalue))
      (set `/Game/BP_New/UI/WB_Dialogue.NPC_Ref` self _output_get)
      (`UserWidget.AddToViewport` (`self.DialogueWidget`) 0))
    (:`then_1`
      (set `self.CurrentSq` 1))
    (:`then_2`
      (set `self.CurrentDialogue` 0))
    (:`then_3`
      (`self.old_ShowNextDialogue` null))
    (:`then_4`
      (`WidgetBlueprintLibrary.SetInputMode_UIOnlyEx` (`GameplayStatics.GetPlayerController` 0) (`self.DialogueWidget`)))))

(fn `PlayAnimation`
  (params (AnimationType :type "/Game/BP_New/Data/E_AnimationType Enum" :default "NewEnumerator0") (MontageRef :type "AnimMontage Object Reference") (DialogueManager :type "/Game/BP_New/System/Manager/BP_DialogueManager Object Reference") (PauseDialogue :type Boolean) (WaitForFinish :type Boolean))
  (bind _dialoguemanagerref (`self.DialogueManagerRef`))
  (bind _returnvalue (`SkeletalMeshComponent.GetAnimInstance` (`self.SkeletalMesh`)))
  (set `self.bIsPauseDialogue` PauseDialogue)
  (set `self.DialogueManagerRef` DialogueManager)
  (`AnimInstance.Montage_Play` _returnvalue MontageRef 1.0 "MontageLength" 0.0 true)
  (if WaitForFinish
    (`KismetSystemLibrary.PrintString` "wait")
    (add `AnimInstance.OnMontageEnded` _returnvalue (`|CreateDelegate` :!event `OnMontageEnded`))
    (else
      (clear `AnimInstance.OnMontageEnded` _returnvalue)
      (set `/Game/BP_New/System/Manager/BP_DialogueManager.bIsEventRunning` false _dialoguemanagerref)
      (`/Game/BP_New/System/Manager/BP_DialogueManager.TryAdvanceDialogue` _dialoguemanagerref))))

(fn `ResumeDialogue`
  (bind _dialoguemanagerref (`self.DialogueManagerRef`))
  (bind _currentdialogueindex (`/Game/BP_New/System/Manager/BP_DialogueManager.CurrentDialogueIndex` _dialoguemanagerref))
  (`/Engine/EditorBlueprintResources/StandardMacros.IsValid` _dialoguemanagerref
    (:`Is Valid`
      (if (`self.bIsPauseDialogue`)
        (`/Engine/EditorBlueprintResources/StandardMacros.IncrementInt` _currentdialogueindex
          (:`  `
            (`UserWidget.AddToViewport` (`/Game/BP_New/System/Manager/BP_DialogueManager.DialogueWidget` _dialoguemanagerref) 0)
            (set `/Game/BP_New/System/Manager/BP_DialogueManager.bIsEventRunning` false _dialoguemanagerref)
            (return)))
        (else
          (set `/Game/BP_New/System/Manager/BP_DialogueManager.bIsEventRunning` false _dialoguemanagerref)
          (`/Engine/EditorBlueprintResources/StandardMacros.IncrementInt` _currentdialogueindex))))))

(fn `UserConstructionScript`)