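; BP_Object_Base is a base work object that can be picked up, rotated and queried for remaining and total defects.
; RotateLeft and RotateRight offset the mesh's roll by RotationAngle and play a timeline meant to lerp the rotation.
; IsRotating guards new turns but is cleared on timeline Update rather than Finished.
; Interaction is allowed only while held, though Interact and ProcessInteract are stubs that perform no action.
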(event `/Game/BP_New/Workobject/BPI_Interactable.Interact`
  (params (Object :type "Actor Object Reference") (HitComponent :type "PrimitiveComponent Object Reference")))

(fn `CanInteract`
  (returns (ReturnValue :type Boolean))
  (if (`self.bIsHolded`)
    (return true)
    (else
      (return false))))

(fn `CanPickup`
  (returns (ReturnValue :type Boolean))
  (return true))

(fn `GetProcessData`
  (returns (`Remain Defects` :type Integer) (`Total Defects` :type Integer))
  (return (`self.RemainDefects`) (`self.TotalDefects`)))

(fn `ProcessInteract`
  (bind _returnvalue (`self.CanInteract`))
  (if (not _returnvalue)
    (return)))

(fn `RotateLeft`
  (if (not (`self.bIsRotating`))
    (bind _output_get (set `self.StartRotation` (`SceneComponent.RelativeRotation` (`self.Object_Mesh`))))
    (set `self.TargetRotation` (`KismetMathLibrary.MakeRotator` (- (.roll _output_get) (`self.RotationAngle`)) (.pitch _output_get) (.yaw _output_get)))
    (set `self.bIsRotating` true)
    (`TimelineComponent.PlayFromStart` (`self.TL_Rotate`))))

(fn `RotateRight`
  (if (not (`self.bIsRotating`))
    (bind _output_get (set `self.StartRotation` (`SceneComponent.RelativeRotation` (`self.Object_Mesh`))))
    (set `self.TargetRotation` (`KismetMathLibrary.MakeRotator` (+ (.roll _output_get) (`self.RotationAngle`)) (.pitch _output_get) (.yaw _output_get)))
    (set `self.bIsRotating` true)
    (`TimelineComponent.PlayFromStart` (`self.TL_Rotate`))))

(fn `UserConstructionScript`)