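; BP_Object_Potato is a pickup minigame object: a potato whose sprouts are removed one by one.
; It starts with a fixed defect count, and interacting while it is held stores the hit component as the target sprout.
; ProcessInteract extends the parent, destroys that component if it is tagged Sprout and decrements the remaining defects.
; The CanInteract checks allow interaction only while defects remain.
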(event `self.ReceiveBeginPlay`
  (bind _output_get (set `self.TotalDefects` 3))
  (set `self.RemainDefects` _output_get))

(event `/Game/BP_New/Workobject/BPI_Interactable.Interact`
  (params (Object :type "Actor Object Reference") (HitComponent :type "PrimitiveComponent Object Reference"))
  (`/Engine/EditorBlueprintResources/StandardMacros.IsValid` HitComponent
    (:`Is Valid`
      (if (`self.bIsHolded`)
        (set `self.TargetSprout` HitComponent)
        (`self.ProcessInteract`)))))

(fn `CanInteract_0`
  (returns (ReturnValue :type Boolean))
  (`parent.CanInteract_0`)
  (if true
    (return (> (`self.RemainDefects`) 0))))

(fn `CanInteract_0_0`
  (returns (ReturnValue :type Boolean))
  (if true
    (return (> (`self.RemainDefects`) 0))))

(fn `CanPickup`
  (returns (ReturnValue :type Boolean))
  (return true))

(fn `ProcessInteract`
  (bind _targetsprout (`self.TargetSprout`))
  (`parent.ProcessInteract`)
  (`/Engine/EditorBlueprintResources/StandardMacros.IsValid` _targetsprout
    (:`Is Valid`
      (if (`ActorComponent.ComponentHasTag` _targetsprout "Sprout")
        (`ActorComponent.K2_DestroyComponent` _targetsprout)
        (`/Engine/EditorBlueprintResources/StandardMacros.DecrementInt` (`self.RemainDefects`))))))

(fn `UserConstructionScript`
  (`parent.UserConstructionScript`))