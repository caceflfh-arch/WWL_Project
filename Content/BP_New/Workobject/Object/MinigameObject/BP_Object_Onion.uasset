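; BP_Object_Onion is a pickup-able minigame onion that is peeled, then cleared of defects while held.
; BeginPlay randomly shows defect components and counts the visible ones.
; Interactions first advance the peel mesh through stages and enable rotation after the last, then destroy hit components tagged "Defact".
; Both peeling and defect removal decrement RemainDefects, while CanInteract passes only before peeling finishes; the peel animation is a print placeholder.
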(event `self.ReceiveBeginPlay`
  (bind _stagemesh (`self.StageMesh`))
  (`parent.ReceiveBeginPlay`)
  (set `self.CurrentStage` 0)
  (`KismetArrayLibrary.Array_Add` _stagemesh "/Game/Prop/Onion/Onion_01.Onion_01")
  (`KismetArrayLibrary.Array_Add` _stagemesh "/Game/Prop/Onion/Onion_02.Onion_02")
  (`StaticMeshComponent.SetStaticMesh` (`self.PeelMesh`) (`|GetArrayItem` _stagemesh))
  (bind _output_get (set `self.DefactComponent` (`|MakeArray` (`self.Defact_0`) (`self.Defact_1`) (`self.Defact_2`))))
  (for _array_element _output_get
    (`SceneComponent.SetVisibility` _array_element (`KismetMathLibrary.RandomBool`) false)
    (if (`SceneComponent.IsVisible` _array_element)
      (`/Engine/EditorBlueprintResources/StandardMacros.IncrementInt` (`self.TotalDefects`)
        (:`  `
          (`/Engine/EditorBlueprintResources/StandardMacros.IncrementInt` (`self.RemainDefects`)))))))

(event `/Game/BP_New/Workobject/BPI_Interactable.Interact`
  (params (Object :type "Actor Object Reference") (HitComponent :type "PrimitiveComponent Object Reference"))
  (`/Engine/EditorBlueprintResources/StandardMacros.IsValid` HitComponent
    (:`Is Valid`
      (if (`self.bIsHolded`)
        (set `self.TargetDefact` HitComponent)
        (`self.ProcessInteract`)))))

(fn `CanInteract`
  (returns (ReturnValue :type Boolean))
  (bind _returnvalue (`parent.CanInteract`))
  (if _returnvalue
    (return (< (`self.CurrentStage`) 2))
    (else
      (return false))))

(fn `CanPickup`
  (returns (ReturnValue :type Boolean))
  (return true))

(fn `ProcessInteract`
  (bind _targetdefact (`self.TargetDefact`))
  (bind _returnvalue (< (`self.CurrentStage`) 2))
  (`parent.ProcessInteract`)
  (if _returnvalue
    (bind _result (`/Engine/EditorBlueprintResources/StandardMacros.IncrementInt` (`self.CurrentStage`))
      (:`  `
        (`/Engine/EditorBlueprintResources/StandardMacros.DecrementInt` (`self.RemainDefects`)
          (:`  `
            (`StaticMeshComponent.SetStaticMesh` (`self.PeelMesh`) (`|GetArrayItem` (`self.StageMesh`) _result))
            (`KismetSystemLibrary.PrintString` "애니메이션:껍질제거")
            (if (not _returnvalue)
              (set `self.bCanRotate` true))))))
    (else
      (`/Engine/EditorBlueprintResources/StandardMacros.IsValid` _targetdefact
        (:`Is Valid`
          (if (`ActorComponent.ComponentHasTag` _targetdefact "Defact")
            (`ActorComponent.K2_DestroyComponent` _targetdefact)
            (`/Engine/EditorBlueprintResources/StandardMacros.DecrementInt` (`self.RemainDefects`))))))))

(fn `UserConstructionScript`
  (`parent.UserConstructionScript`))