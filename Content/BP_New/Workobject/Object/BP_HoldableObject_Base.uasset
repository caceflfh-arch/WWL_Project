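; Base actor for holdable work objects, with stub Action and CanAction functions and a CanPickup that always returns true.
; RotateRight and RotateLeft set a roll target and start a timeline meant to lerp the mesh, whose Update clears the IsRotating guard immediately.
; FlipRight and FlipLeft print a debug string and play flat-grip animations on the player's and left-hand actor's left hands, without moving the object.
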(fn `Action`)

(fn `CanAction`)

(fn `CanPickup`
  (returns (ReturnValue :type Boolean))
  (return true))

(fn `FlipLeft`
  (`KismetSystemLibrary.PrintString` "Hello")
  (bind _returnvalue (`GameplayStatics.GetActorOfClass` "/Game/BP_New/Player/BP_Player_Inhut.BP_Player_Inhut_C"))
  (bind _returnvalue_2 (`GameplayStatics.GetActorOfClass` "/Game/BP_New/Player/Component/BP_LeftHandActor.BP_LeftHandActor_C"))
  (`SkeletalMeshComponent.PlayAnimation` (`/Game/BP_New/Player/BP_Player_Inhut.HoldHand_Left` _returnvalue) "/Game/Defaults/FirstPersonArms/Character/Mesh/AN_FlatGrip_Flip.AN_FlatGrip_Flip" false)
  (`SkeletalMeshComponent.PlayAnimation` (`/Game/BP_New/Player/Component/BP_LeftHandActor.WorkHand_Left` _returnvalue_2) "/Game/Defaults/FirstPersonArms/Character/Mesh/AN_FlatGrip_Flip.AN_FlatGrip_Flip" false))

(fn `FlipRight`
  (`KismetSystemLibrary.PrintString` "Hello")
  (bind _returnvalue (`GameplayStatics.GetActorOfClass` "/Game/BP_New/Player/BP_Player_Inhut.BP_Player_Inhut_C"))
  (bind _returnvalue_2 (`GameplayStatics.GetActorOfClass` "/Game/BP_New/Player/Component/BP_LeftHandActor.BP_LeftHandActor_C"))
  (`SkeletalMeshComponent.PlayAnimation` (`/Game/BP_New/Player/BP_Player_Inhut.HoldHand_Left` _returnvalue) "/Game/Defaults/FirstPersonArms/Character/Mesh/AN_FlatGrip.AN_FlatGrip" false)
  (`SkeletalMeshComponent.PlayAnimation` (`/Game/BP_New/Player/Component/BP_LeftHandActor.WorkHand_Left` _returnvalue_2) "/Game/Defaults/FirstPersonArms/Character/Mesh/AN_FlatGrip.AN_FlatGrip" false))

(fn `RotateLeft`
  (if (not (`self.bIsRotating`))
    (bind _output_get (set `self.StartRotation` (`SceneComponent.RelativeRotation` (`self.Object_Mesh`))))
    (set `self.TargetRotation` (`KismetMathLibrary.MakeRotator` (- (.roll _output_get) (`self.RotationAngle`)) (.pitch _output_get) (.yaw _output_get)))
    (set `self.bIsRotating` true)
    (`TimelineComponent.PlayFromStart` (`self.TL_Rotate`))))

(fn `RotateRight`
  (if (not (`self.bIsRotating`))
    (bind _output_get (set `self.StartRotation` (`SceneComponent.RelativeRotation` (`self.Object_Mesh`))))
    (set `self.TargetRotation` (`KismetMathLibrary.MakeRotator` (+ (.roll _output_get) (`self.RotationAngle`)) (.pitch _output_get) (.yaw _output_get)))
    (set `self.bIsRotating` true)
    (`TimelineComponent.PlayFromStart` (`self.TL_Rotate`))))

(fn `UserConstructionScript`)