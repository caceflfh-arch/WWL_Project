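; Base table Blueprint with a serving zone whose contents are gathered when a serving is submitted.
; Submit resets the total score, calls EvaluateServing and then flags the table as submitting.
; EvaluateServing collects overlapping BP_Object_Base actors into ValidObjects without clearing it first, then prints their names.
; No score is calculated yet, the event graph is empty, and output is only debug prints.
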(fn `EvaluateServing`
  (set `self.DetectedActors` (`PrimitiveComponent.GetOverlappingActors` (`self.ServingZone`) null))
  (for _array_element (`self.DetectedActors`)
    (bind _asbp_object_base (cast `/Game/BP_New/Workobject/Object/BP_Object_Base` _array_element))
    (`KismetArrayLibrary.Array_Add` (`self.ValidObjects`) _asbp_object_base))
  (for _array_element_2 (`self.ValidObjects`)
    (`KismetSystemLibrary.PrintString` (`KismetSystemLibrary.GetDisplayName` _array_element_2)))
  (`KismetSystemLibrary.PrintString` "Array 등록 완료"))

(fn `Submit`
  (set `self.TotalScore` 0.0)
  (`self.EvaluateServing`)
  (set `self.bIsSubmitting` true)
  (`KismetSystemLibrary.PrintString` "Submit Done")
  (return))

(fn `UserConstructionScript`)