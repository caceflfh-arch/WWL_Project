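; BP_Table_ServingFood is a food-serving table work object that grades the objects submitted on it.
; Submit runs the parent logic, then adds each valid object's percentage of removed defects, read from its process data, to TotalScore.
; It prints the average but picks one of two grades by comparing the accumulated total, not the average, to a threshold, then prints the grade.
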(event `self.ReceiveBeginPlay`)

(fn `Submit`
  (locals (Grade :type "/Game/BP_New/Data/E_OverallGrade Enum"))
  (bind _validobjects (`self.ValidObjects`))
  (`parent.Submit`)
  (for _array_element _validobjects
    (bind (_remain_defects _total_defects) (`/Game/BP_New/Workobject/Object/MinigameObject/BP_MinigameObject_Base.GetProcessData` _array_element))
    (set `self.TotalScore` (+ (`self.TotalScore`) (* (- 1.0 (/ (`KismetMathLibrary.Conv_IntToDouble` _remain_defects) _total_defects)) 100.0))))
  (`KismetSystemLibrary.PrintString` (`KismetStringLibrary.Concat_StrStr` "TotalScore : " (`KismetStringLibrary.Conv_DoubleToString` (/ (`self.TotalScore`) (`KismetArrayLibrary.Array_Length` _validobjects)))))
  (if (> (`self.TotalScore`) 80.0)
    (set `local.Grade` "NewEnumerator0")
    (else
      (set `local.Grade` "NewEnumerator1")))
  (`KismetSystemLibrary.PrintString` (`KismetStringLibrary.Concat_StrStr` "Submit! Grade : " (`|GetEnumeratorNameAsString` (`local.Grade`)))))

(fn `UserConstructionScript`
  (`parent.UserConstructionScript`))