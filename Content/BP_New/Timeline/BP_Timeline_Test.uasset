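; Test cinematic event actor that the dialogue manager reference is handed to, playing a short scripted scene during dialogue.
; PlayCinematic stores the manager and pause flag, then runs a timeline whose track threshold, checked against a Spawned flag, spawns BP_TestPerson at a hardcoded transform.
; After starting a looping walk animation and waiting, it clears the manager's event state, advances the index, re-adds the widget if paused and calls PlayNext.
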(event `self.ReceiveBeginPlay`)

(event `TimelinePlay`
  ;[1 1 1] Dummy
  (bind (_direction _newtrack_0) (`Timeline|Timeline_Test`) ; test
    (:`Update`
      (if (!= (`self.bSpawned`) (> _newtrack_0 0.2))
        (bind _returnvalue (`|SpawnActorFromClass` "/Game/BP_New/Timeline/Actor/BP_TestPerson.BP_TestPerson_C" (`KismetMathLibrary.MakeTransform` (350.0 125.0 0.0) (struct :`Yaw` 180.0)) "Undefined" "MultiplyWithRoot" null null))
        (bind _output_get (set `self. SpawnActor` _returnvalue))
        (set `self.bSpawned` true)
        (`KismetSystemLibrary.Delay` 0.1)
        (`SkeletalMeshComponent.PlayAnimation` (`/Game/BP_New/Timeline/Actor/BP_TestPerson.SkeletalMesh` _output_get) "/Game/Character/TestNPC/Test_Walk.Test_Walk" true)
        (`KismetSystemLibrary.Delay` 3.0)
        (`self.EndTimeline`)
        (`/Game/BP_New/System/Manager/BP_DialogueManager.PlayNext` (`self.DialogueManagerRef`))))))

(fn `EndTimeline`
  (bind _dialoguemanagerref (`self.DialogueManagerRef`))
  (bind _currentdialogueindex (`/Game/BP_New/System/Manager/BP_DialogueManager.CurrentDialogueIndex` _dialoguemanagerref))
  (`/Engine/EditorBlueprintResources/StandardMacros.IsValid` _dialoguemanagerref
    (:`Is Valid`
      (if (`self.bIsPauseDialogue`)
        (`/Engine/EditorBlueprintResources/StandardMacros.IncrementInt` _currentdialogueindex
          (:`  `
            (`UserWidget.AddToViewport` (`/Game/BP_New/System/Manager/BP_DialogueManager.DialogueWidget` _dialoguemanagerref) 0)
            (set `/Game/BP_New/System/Manager/BP_DialogueManager.bIsEventRunning` false _dialoguemanagerref)))
        (else
          (set `/Game/BP_New/System/Manager/BP_DialogueManager.bIsEventRunning` false _dialoguemanagerref)
          (`/Engine/EditorBlueprintResources/StandardMacros.IncrementInt` _currentdialogueindex))))))

(fn `PlayCinematic`
  (params (DialogueManager :type "/Game/BP_New/System/Manager/BP_DialogueManager Object Reference") (bIsPauseDialogue :type Boolean))
  (set `self.bIsPauseDialogue` bIsPauseDialogue)
  (set `self.DialogueManagerRef` DialogueManager)
  (`self.TimelinePlay`))

(fn `UserConstructionScript`)