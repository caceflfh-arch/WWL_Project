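; BP_GameManager is a game manager actor that starts the current day of a day-based, dialogue-driven game.
; On BeginPlay it prints a load-data placeholder, finds BP_DialogueManager and calls StartDay, which handles only day 1 by starting dialogue from DT_Day1 at a debug sequence.
; UnlockNextDay increments the unlocked day count, while SetFlag and GetFlag are unfinished stubs.
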(event `self.ReceiveBeginPlay`
  (`KismetSystemLibrary.PrintString` "(Load Data)")
  (bind _returnvalue (`GameplayStatics.GetActorOfClass` "/Game/BP_New/System/Manager/BP_DialogueManager.BP_DialogueManager_C"))
  (set `self.DialogueManagerRef` _returnvalue)
  (`self.StartDay` (`self.CurrentDay`)))

(fn `GetFlag`)

(fn `SetFlag`
  (params (FlagName :type Name))
  (returns (ReturnValue :type Boolean))
  (return false))

(fn `StartDay`
  (params (DayIndex :type Integer))
  (switch `int` DayIndex
    (:`1`
      (set `self.CurrentDialogueTable` "/Game/BP_New/Data/DT_Day1.DT_Day1")
      (`/Game/BP_New/System/Manager/BP_DialogueManager.StartDialogue` (`self.DialogueManagerRef`) (`self.DebugSq`) null "NewEnumerator0" (`self.CurrentDialogueTable`) DayIndex))))

(fn `UnlockNextDay`
  (`/Engine/EditorBlueprintResources/StandardMacros.IncrementInt` (`self.UnlockedDays`)))

(fn `UserConstructionScript`)