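; BP_CarrotZone is a zone actor that spawns carrots and keeps them organized in slots.
; On BeginPlay it initializes slots from CarrotSlotsRoot, spawns SpawnCount BP_Carrot actors at its own transform, adds each to a slot, then compacts the slots.
; AddToSlotObject and RemoveToSlotObject wrap the generic AddObject and RemoveObject slot functions, passing in the carrot slot and object arrays.
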(event `self.ReceiveBeginPlay`
  (`parent.ReceiveBeginPlay`)
  (`self.InitializeSlots` (`self.CarrotSlotsRoot`) (`self.CarrotSlots`) (`self.CarrotObjects`))
  (`self.SpawnCarrots`))

(fn `AddToSlotObject`
  (params (ObjectToAdd :type "/Game/Blueprints/Base/BP_WorkObject_Base Object Reference"))
  (`self.AddObject` ObjectToAdd (`self.CarrotSlots`) (`self.CarrotObjects`)))

(fn `RemoveToSlotObject`
  (params (ObjectToRemove :type "/Game/Blueprints/Base/BP_WorkObject_Base Object Reference"))
  (`self.RemoveObject` ObjectToRemove (`self.CarrotSlots`) (`self.CarrotObjects`)))

(fn `SpawnCarrots`
  (for _ (range (`self.SpawnCount`))
    (bind _returnvalue (`|SpawnActorFromClass` "/Game/Blueprints/BP_Carrot.BP_Carrot_C" (`self.GetTransform`) "Undefined" "MultiplyWithRoot" null null))
    (`self.AddObject` _returnvalue (`self.CarrotSlots`) (`self.CarrotObjects`)))
  (`self.CompactSlots` (`self.CarrotObjects`) (`self.CarrotSlots`)))

(fn `UserConstructionScript`
  (`parent.UserConstructionScript`))