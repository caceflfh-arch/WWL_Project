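; BP_ScoreManager scores a submission of Potato, Carrot and Garlic objects through a single EvaluateSubmission function.
; The function loops over the submitted objects, summing quality scores and counting the total and each type.
; It then derives an average quality, guarded against empty submissions, and sorts the total count into one of three quantity result tiers.
; The event graph and construction script hold no logic.
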(fn `EvaluateSubmission`
  (params (SubmittedObjects :type "Array of /Game/Blueprints/Base/BP_WorkObject_Base Object Reference"))
  (returns (EvaluationResult :type "/Game/Blueprints/Struct/FS_EvaluationResult Structure"))
  (locals (AverageQuality :type "Float (double-precision)") (QuantityResult :type "/Game/Blueprints/Enum/ReactionType/E_IngredientQuantity Enum"))
  (set `self.TotalCount` 0)
  (set `self.TotalQualityScore` 0.0)
  (set `self.PotatoCount` 0)
  (set `self.CarrotCount` 0)
  (set `self.GarlicCount` 0)
  (for _array_element SubmittedObjects
    (`/Engine/EditorBlueprintResources/StandardMacros.IncrementFloat` (`KismetMathLibrary.Conv_IntToDouble` (`self.TotalCount`))
      (:`  `
        (set `self.TotalQualityScore` (+ (`/Game/Blueprints/Base/BP_WorkObject_Base.QualityScore` _array_element) (`self.TotalQualityScore`)))
        (`/Engine/EditorBlueprintResources/StandardMacros.IncrementInt` (`self.TotalCount`)
          (:`  `
            (switch `/Game/Blueprints/Enum/E_WorkObjectType` (`self.WokrObjectType`)
              (:`NewEnumerator0`
                (`/Engine/EditorBlueprintResources/StandardMacros.IncrementInt` (`self.PotatoCount`)
                  (:`  `
                    _)))
              (:`NewEnumerator1`
                (`/Engine/EditorBlueprintResources/StandardMacros.IncrementInt` (`self.CarrotCount`)
                  (:`  `
                    _)))
              (:`NewEnumerator2`
                (`/Engine/EditorBlueprintResources/StandardMacros.IncrementInt` (`self.GarlicCount`)
                  (:`  `
                    _))))
            (return))))))
  (if (> (`self.TotalCount`) 0)
    (set `local.AverageQuality` (/ (`self.TotalQualityScore`) (`self.TotalCount`)))
    (else
      (set `local.AverageQuality` 0.0)))
  (if (< (`self.TotalCount`) 2)
    (set `local.QuantityResult` "NewEnumerator5")
    (elif (>= (`self.TotalCount`) 4)
      (set `local.QuantityResult` "NewEnumerator7")
      (else
        (set `local.QuantityResult` "NewEnumerator6")))))

(fn `UserConstructionScript`)