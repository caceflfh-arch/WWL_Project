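; BP_Carrot is a carrot Blueprint whose wound or sprout components are removed by work hits.
; HandleWoundHit destroys each valid hit component, decrements SproutCount, then sets a completion flag and prints a Korean "wound removal complete" message once none remain.
; A Sprout tag check is left unwired, so any valid component passed in counts.
; The event graph is empty, and old_OnWorkHit only forwards to HandleWoundHit.
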(fn `HandleWoundHit`
  (params (HitComp :type "PrimitiveComponent Object Reference"))
  (`/Engine/EditorBlueprintResources/StandardMacros.IsValid` HitComp
    (:`Is Valid`
      (`ActorComponent.K2_DestroyComponent` HitComp)
      (`/Engine/EditorBlueprintResources/StandardMacros.DecrementInt` (`self.SproutCount`)
        (:`  `
          (if (<= (`self.SproutCount`) 0)
            (set `self.bIsCompleted_0` true)
            (`KismetSystemLibrary.PrintString` "상처제거완료")))))))

(fn `old_OnWorkHit`
  (params (OnWorkHit :type "PrimitiveComponent Object Reference"))
  (`self.HandleWoundHit` OnWorkHit))

(fn `UserConstructionScript`)