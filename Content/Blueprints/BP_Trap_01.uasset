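; BP_Trap_01 is a trap actor that sends the player to Map_Hut when a Character overlaps its TrapTrigger.
; The overlap disables player input, plays the CompileFailed sound and creates an M_FadeOut dynamic instance, which is left unused.
; A timeline writes FadeAmount to the MPC_Fade parameter collection.
; That timeline's Update also calls OpenLevel and starts a second fade timeline, rather than waiting for completion.
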(event `self.TrapTrigger.OnComponentBeginOverlap`
  (params (OverlappedComponent :type "PrimitiveComponent Object Reference") (OtherActor :type "Actor Object Reference") (OtherComp :type "PrimitiveComponent Object Reference") (OtherBodyIndex :type Integer) (bFromSweep :type Boolean) (SweepResult :type "HitResult Structure (by ref)"))
  ;[1 1 1] 캐릭터 충돌 판정
  (cast `Character` OtherActor)
  ;[1 1 1] 입력 중단
  (`self.DisableInput` (`GameplayStatics.GetPlayerPawn` 0) null)
  ;[1 1 1] 사운드 재생
  (`GameplayStatics.PlaySoundAtLocation` "/Engine/EditorSounds/Notifications/CompileFailed.CompileFailed" (`self.K2_GetActorLocation`) (struct) 1.0 1.0 0.0 null null null null)
  ;[1 1 1] Fadeout Material 불러오기
  (`KismetMaterialLibrary.CreateDynamicMaterialInstance` "/Game/Materials/PostProcess/M_FadeOut.M_FadeOut")
  ;[1 1 1] Fadeout Material 제어 타임라인
  (bind (_direction _fadealpha) (`Timeline|Timeline`)
    (:`Update`
      (`KismetMaterialLibrary.SetScalarParameterValue` "/Game/Materials/PostProcess/MPC/MPC_Fade.MPC_Fade" "FadeAmount" _fadealpha)
      ;[1 1 1] 레벨 이동
      (`GameplayStatics.OpenLevel` "Map_Hut")
      ;[1 1 1] Fadeout Material 제어 타임라인
      (bind (_direction_2 _fadealpha_2) (`Timeline|Timeline_0`)
        (:`Update`
          (`KismetMaterialLibrary.SetScalarParameterValue` "/Game/Materials/PostProcess/MPC/MPC_Fade.MPC_Fade" "FadeAmount" _fadealpha_2))))))

(fn `UserConstructionScript`)