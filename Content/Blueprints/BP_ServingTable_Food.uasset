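; Serving table Blueprint for food that sorts ingredients into separate potato and carrot serving zones.
; On BeginPlay it casts the two Child Actor components to their zone classes and caches the references.
; AddIngredient switches on the ingredient's WorkObjectType and passes it to the matching zone's AddToSlotObject.
; The potato branch also prints a leftover debug string.
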(event `self.ReceiveBeginPlay`
  (bind _asbp_serving_zone_potato (cast `/Game/Blueprints/BP_ServingZone_Potato` (`ChildActorComponent.ChildActor` (`self.PotatoZone`))))
  (set `self.PotatoZoneRef` _asbp_serving_zone_potato)
  (bind _asbp_serving_zone_carrot (cast `/Game/Blueprints/BP_ServingZone_Carrot` (`ChildActorComponent.ChildActor` (`self.CarrotZone`))))
  (set `self.CarrotZoneRef` _asbp_serving_zone_carrot))

(fn `AddIngredient`
  (params (Ingredient :type "/Game/Blueprints/Base/BP_WorkObject_Base Object Reference"))
  (switch `/Game/Blueprints/Enum/E_WorkObjectType` (`/Game/Blueprints/Base/BP_WorkObject_Base.WorkObjectType` Ingredient)
    (:`NewEnumerator0`
      (`KismetSystemLibrary.PrintString` "Hello")
      (`self.AddToSlotObject` (`self.PotatoZoneRef`) Ingredient))
    (:`NewEnumerator1`
      (`self.AddToSlotObject` (`self.CarrotZoneRef`) Ingredient))))

(fn `UserConstructionScript`)