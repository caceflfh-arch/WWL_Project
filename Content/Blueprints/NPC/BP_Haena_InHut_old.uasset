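; BP_Haena_InHut_old is an NPC Blueprint for Haena in the hut that shows dialogue from DT_HaenainHut_Dialogue.
; ShowDialogue resets the counter, opens WB_Dialogue and sets UI-only input, passing the widget reference before assigning it.
; NextDialogue increments the counter and prints matching rows, but clears the widget reference before setting its text.
; Both scan every row, matching Sq by bitwise AND with the counter rather than equality.
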(event `ShowDialogue`
  (bind _output_get (set `self.CurrentDialogue` 1))
  (bind _returnvalue (`|CreateWidget` "/Game/Blueprints/UI/WB_Dialogue.WB_Dialogue_C" (`GameplayStatics.GetPlayerController` 0) self))
  (`WidgetBlueprintLibrary.SetInputMode_UIOnlyEx` (`GameplayStatics.GetPlayerController` 0) (`self.DialogueWidgetRef`))
  (bind _output_get_2 (set `self.DialogueWidgetRef` _returnvalue))
  (`UserWidget.AddToViewport` _output_get_2 0)
  (bind _outrownames (`DataTableFunctionLibrary.GetDataTableRowNames` "/Game/DataTables/DT_HaenainHut_Dialogue.DT_HaenainHut_Dialogue"))
  (for _array_element _outrownames
    (bind _returnvalue_2 (`|GetDataTableRow` "/Game/DataTables/DT_HaenainHut_Dialogue.DT_HaenainHut_Dialogue" _array_element)
      (:`then`
        (bind (_sq _dialog _speakername _dialoguetext _playerchoice _lastdialogue _dialoguetext_2) (break `/Game/Blueprints/FS_Dialogue` _returnvalue_2))
        (if (`KismetMathLibrary.Conv_IntToBool` (`KismetMathLibrary.And_IntInt` _sq _output_get))
          (`/Game/Blueprints/UI/WB_Dialogue.SetDialogueText` (`self.DialogueWidgetRef`) _dialoguetext_2))))))

(event `NextDialogue`
  (bind _result (`/Engine/EditorBlueprintResources/StandardMacros.IncrementFloat` (`KismetMathLibrary.Conv_IntToDouble` (`self.CurrentDialogue`)))
    (:`  `
      (bind _output_get (set `self.CurrentDialogue` (`KismetMathLibrary.FTrunc` _result)))
      (bind _outrownames (`DataTableFunctionLibrary.GetDataTableRowNames` "/Game/DataTables/DT_HaenainHut_Dialogue.DT_HaenainHut_Dialogue"))
      (for _array_element _outrownames
        (bind _returnvalue (`|GetDataTableRow` "/Game/DataTables/DT_HaenainHut_Dialogue.DT_HaenainHut_Dialogue" _array_element)
          (:`then`
            (bind (_sq _dialog _speakername _dialoguetext _playerchoice _lastdialogue _dialoguetext_2) (break `/Game/Blueprints/FS_Dialogue` _returnvalue))
            (if (`KismetMathLibrary.Conv_IntToBool` (`KismetMathLibrary.And_IntInt` _sq _output_get))
              (`KismetSystemLibrary.PrintString` (`KismetTextLibrary.Conv_TextToString` _dialoguetext_2))
              (bind _output_get_2 (set `self.DialogueWidgetRef` null))
              (`/Game/Blueprints/UI/WB_Dialogue.SetDialogueText` _output_get_2 _dialoguetext_2))))))))

(fn `UserConstructionScript`)