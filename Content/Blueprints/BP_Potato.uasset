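; BP_Potato is a work object for potato trimming, with sprouts to remove as work points.
; On BeginPlay it spawns a random number of BP_WorkPoint_Potato actors, attaches them to socket components and sets itself as their parent.
; ReportPointCompleted counts finished points against MaxSproutCount, which is rolled separately from the spawn count, and prints completion.
; An older wound-hit path destroys hit components and decrements that same maximum.
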(event `self.ReceiveBeginPlay`
  (bind _returnvalue (`KismetMathLibrary.RandomIntegerInRange` 2 5))
  (bind _workpointsockets (`self.WorkPointSockets`))
  (set `self.SpawnSproutCount` _returnvalue)
  (set `self.MaxSproutCount` _returnvalue)
  (`KismetArrayLibrary.Array_Add` _workpointsockets (`self.WP_Slot_0`))
  (`KismetArrayLibrary.Array_Add` _workpointsockets (`self.WP_Slot_1`))
  (`KismetArrayLibrary.Array_Add` _workpointsockets (`self.WP_Slot_2`))
  (`KismetArrayLibrary.Array_Add` _workpointsockets (`self.WP_Slot_3`))
  (`KismetArrayLibrary.Array_Add` _workpointsockets (`self.WP_Slot_4`))
  (for _index (range (`self.SpawnSproutCount`))
    (bind _output (`|GetArrayItem` (`self.WorkPointSockets`) _index))
    (bind _returnvalue_2 (`|SpawnActorFromClass` "/Game/Blueprints/BP_WorkPoint_Potato.BP_WorkPoint_Potato_C" (`SceneComponent.K2_GetComponentToWorld` _output) "Undefined" "MultiplyWithRoot" null null))
    (set `/Game/Blueprints/Base/BP_WorkPoint_Base.ParentWorkObject` self _returnvalue_2)
    (`self.K2_AttachToComponent` _returnvalue_2 _output "None" "SnapToTarget" "SnapToTarget" "KeepRelative" false)))

(fn `HandleWoundHit`
  (params (HitComp :type "PrimitiveComponent Object Reference"))
  (`/Engine/EditorBlueprintResources/StandardMacros.IsValid` HitComp
    (:`Is Valid`
      (`ActorComponent.K2_DestroyComponent` HitComp)
      (`/Engine/EditorBlueprintResources/StandardMacros.DecrementInt` (`self.MaxSproutCount`)
        (:`  `
          (if (<= (`self.MaxSproutCount`) 0)
            (set `self.bIsCompleted_0` true)
            (`KismetSystemLibrary.PrintString` "상처제거완료")))))))

(fn `old_OnWorkHit`
  (params (OnWorkHit :type "PrimitiveComponent Object Reference"))
  (`self.HandleWoundHit` OnWorkHit))

(fn `ReportPointCompleted`
  (`/Engine/EditorBlueprintResources/StandardMacros.IncrementInt` (`self.CompletedSproutCount`)
    (:`  `
      (if (>= (`self.CompletedSproutCount`) (`self.MaxSproutCount`))
        (`KismetSystemLibrary.PrintString` "감자손질완료")))))

(fn `UserConstructionScript`)