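; BP_WorkPoint_Base is a base Blueprint for an interactable work point that belongs to a parent work object.
; HandleInteract calls CompletePoint, which runs once: it sets IsCompleted, destroys the actor, then calls CalculateQuality on ParentWorkObject.
; CanInteract allows interaction until completion, and GetWorkMesh exposes the point's mesh.
; The OnInteract event and the other EventGraph events are empty.
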(event `self.ReceiveBeginPlay`)

(event `/Game/Blueprints/Interface/BPI_Interactable.OnInteract`)

(fn `CanInteract`
  (returns (ReturnValue :type Boolean))
  (return (not (`self.bIsCompleted`))))

(fn `CompletePoint`
  (if (not (`self.bIsCompleted`))
    (set `self.bIsCompleted` true)
    (`self.K2_DestroyActor`)
    (`/Game/Blueprints/Base/BP_WorkObject_Base.CalculateQuality` (`self.ParentWorkObject`))))

(fn `GetWorkMesh`
  (returns (WorkMesh :type "StaticMeshComponent Object Reference"))
  (return (`self.WorkMesh`)))

(fn `HandleInteract`
  (`self.CompletePoint`))

(fn `UserConstructionScript`)