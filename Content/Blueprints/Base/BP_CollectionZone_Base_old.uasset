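; Base collection zone actor that holds work objects in tagged slot components and tracks itself as their ParentZone.
; On BeginPlay it gathers "Slot"-tagged components and fills them with spawned, randomly rotated objects.
; Older functions store and remove objects through that slot array.
; A separate Slots/StoredObjects set adds objects to the first empty slot and compacts on removal, but BeginPlay never initializes it.
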(event `self.ReceiveBeginPlay`
  (bind _returnvalue (`KismetMathLibrary.RandomFloatInRange` 0.0 360.0))
  (`KismetArrayLibrary.Array_Resize` (`self.SlotObjects`) 5)
  (`|ExecutionSequence`
    (:`then_0`
      (for _array_element (`self.K2_GetComponentsByClass` "/Script/Engine.SceneComponent")
        (if (`ActorComponent.ComponentHasTag` _array_element "Slot")
          (`KismetArrayLibrary.Array_Add` (`self.Slotpoint`) _array_element))))
    (:`then_1`
      (for _index (range (`self.MaxCount`))
        (bind _output (`|GetArrayItem` (`self.Slotpoint`) _index))
        (bind _returnvalue_2 (`|SpawnActorFromClass` (`self.SpawnObjectClass`) (`KismetMathLibrary.MakeTransform` (.location (`SceneComponent.K2_GetComponentToWorld` _output)) (`KismetMathLibrary.MakeRotator` _returnvalue _returnvalue _returnvalue) (.scale (`SceneComponent.K2_GetComponentToWorld` _output))) "AlwaysSpawn" "MultiplyWithRoot" null null))
        (`self.K2_AttachToComponent` _returnvalue_2 _output "None" "SnapToTarget" "KeepWorld" "KeepWorld" false)
        (set `/Game/Blueprints/Base/BP_WorkObject_Base.ParentZone` self _returnvalue_2)
        (`KismetArrayLibrary.Array_Set` (`self.SlotObjects`) _index _returnvalue_2)))))

(fn `AddObject`
  (params (Object :type "/Game/Blueprints/Base/BP_WorkObject_Base Object Reference"))
  (bind _index (`self.Index`))
  (bind _index_2 (`self.GetEmptySlotIndex`))
  (bind _output_get (set `self.Index` _index_2))
  (if (>= _output_get 0)
    (`KismetArrayLibrary.Array_Set` (`self.StoredObjects`) _index Object)
    (`self.K2_AttachToComponent` Object (`|GetArrayItem` (`self.Slots`) _index) "None" "SnapToTarget" "SnapToTarget" "KeepRelative" true)
    (set `/Game/Blueprints/Base/BP_WorkObject_Base.ParentZone` self Object)))

(fn `AttachObjectToSlot`)

(fn `CompactSlots`
  (bind _storedobjects (`self.StoredObjects`))
  (bind _writeindex (`self.WriteIndex`))
  (for _index (range (`KismetArrayLibrary.Array_Length` (`self.StoredObjects`)))
    (`KismetSystemLibrary.PrintString` "Hello")
    (bind _output (`|GetArrayItem` _storedobjects _index))
    (`/Engine/EditorBlueprintResources/StandardMacros.IsValid` _output
      (:`Is Valid`
        (`KismetArrayLibrary.Array_Set` _storedobjects _writeindex _output)
        (`self.K2_AttachToComponent` _output (`|GetArrayItem` (`self.Slots`) _writeindex) "None" "SnapToTarget" "SnapToTarget" "KeepRelative" true)
        (set `self.WriteIndex` (+ _writeindex 1))))))

(fn `GetEmptySlotIndex`
  (returns (Index :type Integer))
  (for _index (range (`KismetArrayLibrary.Array_Length` (`self.Slots`)))
    (`/Engine/EditorBlueprintResources/StandardMacros.IsValid` (`|GetArrayItem` (`self.StoredObjects`) _index)
      (:`Is Not Valid`
        (return _index))))
  (return -1))

(fn `InitializeSlots`
  (params (SlotRoot :type "SceneComponent Object Reference") (SlotArray :type "Array of SceneComponent Object Reference") (SlotObjects :type "Array of SceneComponent Object Reference"))
  (`KismetArrayLibrary.Array_Clear` SlotArray)
  (for _array_element (`SceneComponent.GetChildrenComponents` SlotRoot false)
    (`KismetArrayLibrary.Array_Add` SlotArray _array_element)
    (`KismetArrayLibrary.Array_Resize` SlotObjects (`KismetArrayLibrary.Array_Length` SlotArray))))

(fn `RemoveFromSlot_old`
  (params (WorkObject :type "/Game/Blueprints/Base/BP_WorkObject_Base Object Reference"))
  (bind _slotobjects (`self.SlotObjects`))
  (for _index (range (`KismetArrayLibrary.Array_Length` (`self.SlotObjects`)))
    (if (== (`|GetArrayItem` _slotobjects _index) WorkObject)
      (`KismetArrayLibrary.Array_Set` _slotobjects _index)
      (break))))

(fn `RemoveObject`
  (params (Object :type "/Game/Blueprints/Base/BP_WorkObject_Base Object Reference"))
  (bind _returnvalue (`KismetArrayLibrary.Array_Find` (`self.StoredObjects`) Object))
  (if (>= _returnvalue 0)
    (`KismetArrayLibrary.Array_Set` (`self.StoredObjects`) _returnvalue)
    (set `/Game/Blueprints/Base/BP_WorkObject_Base.ParentZone` null Object)
    (`self.CompactSlots`)))

(fn `StoreObject_old`
  (params (WorkObject :type "/Game/Blueprints/Base/BP_WorkObject_Base Object Reference"))
  (bind _workobject (`local.WorkObject`))
  (bind _slotobjects (`self.SlotObjects`))
  (for _index (range (`KismetArrayLibrary.Array_Length` _slotobjects))
    (`/Engine/EditorBlueprintResources/StandardMacros.IsValid` (`|GetArrayItem` (`self.SlotObjects`) _index)
      (:`Is Not Valid`
        (`self.K2_DetachFromActor` _workobject "KeepWorld" "KeepWorld" "KeepWorld")
        (`self.K2_AttachToComponent` _workobject (`|GetArrayItem` (`self.Slotpoint`) _index) "None" "SnapToTarget" "KeepRelative" "KeepWorld" true)
        (`KismetArrayLibrary.Array_Set` _slotobjects _index _workobject)
        (break)))))

(fn `UserConstructionScript`)