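; Potato serving zone that stocks itself with potato actors and keeps them arranged in slots.
; On BeginPlay it initializes slots from a root component, then spawns a set number of BP_Potato actors, adds each to a slot and compacts the arrangement.
; Add and remove functions pass the potato slot and object arrays to shared slot helpers, which are defined outside this graph.
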(event `self.ReceiveBeginPlay`
  (`parent.ReceiveBeginPlay`)
  (`self.InitializeSlots` (`self.PotatoSlotsRoot`) (`self.PotatoSlots`) (`self.PotatoObjects`))
  (`self.SpawnPotatoes`))

(fn `AddToSlotObject`
  (params (ObjectToAdd :type "/Game/Blueprints/Base/BP_WorkObject_Base Object Reference"))
  (`self.AddObject` ObjectToAdd (`self.PotatoSlots`) (`self.PotatoObjects`)))

(fn `RemoveToSlotObject`
  (params (ObjectToRemove :type "/Game/Blueprints/Base/BP_WorkObject_Base Object Reference"))
  (`self.RemoveObject` ObjectToRemove (`self.PotatoSlots`) (`self.PotatoObjects`)))

(fn `SpawnPotatoes`
  (for _ (range (`self.SpawnCount`))
    (bind _returnvalue (`|SpawnActorFromClass` "/Game/Blueprints/BP_Potato.BP_Potato_C" (`self.GetTransform`) "Undefined" "MultiplyWithRoot" null null))
    (`self.AddObject` _returnvalue (`self.PotatoSlots`) (`self.PotatoObjects`)))
  (`self.CompactSlots` (`self.PotatoObjects`) (`self.PotatoSlots`)))

(fn `UserConstructionScript`
  (`parent.UserConstructionScript`))