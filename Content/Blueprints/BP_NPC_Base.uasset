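; Base NPC Blueprint that runs a data-table-driven dialogue when its ShowDialogue event fires.
; StartDialogue creates a WB_Dialogue widget linked back to the NPC, resets sequence and line counters, shows the first line and switches to UI-only input.
; ShowNextDialogue, gated by IsInteracting, increments the line and scans DT_HaenainHut_Dialogue for the matching row.
; A row flagged LastDialogue immediately triggers EndDialogue, removing the widget and restoring game input.
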(event `ShowDialogue`
  (`self.StartDialogue`))

(fn `EndDialogue`
  (bind _returnvalue (`GameplayStatics.GetPlayerController` 0))
  (`Widget.RemoveFromParent` (`self.DialogueWidget`))
  (`WidgetBlueprintLibrary.SetInputMode_GameOnly` _returnvalue)
  (set `PlayerController.bShowMouseCursor` false _returnvalue)
  (set `self.DialogueWidget` null))

(fn `ShowNextDialogue`
  (if (== (`self.bIsInteracting`) false)
    (`/Engine/EditorBlueprintResources/StandardMacros.IsValid` (`self.DialogueWidget`)
      (:`Is Valid`
        (bind _output_get (set `self.CurrentDialogue` (`self.CurrentDialogue`)))
        (`/Engine/EditorBlueprintResources/StandardMacros.IncrementInt` _output_get
          (:`  `
            (bind _outrownames (`DataTableFunctionLibrary.GetDataTableRowNames` "/Game/DataTables/DT_HaenainHut_Dialogue.DT_HaenainHut_Dialogue"))
            (for _array_element _outrownames
              (bind _returnvalue (`|GetDataTableRow` "/Game/DataTables/DT_HaenainHut_Dialogue.DT_HaenainHut_Dialogue" _array_element)
                (:`then`
                  (bind _output_get_2 (set `self.TempRow` _returnvalue))
                  (bind (_sq _dialog _speakername _dialoguetext _playerchoice _lastdialogue) (break `/Game/Blueprints/Struct/FS_Dialogue` _output_get_2))
                  (if (`KismetMathLibrary.Conv_IntToBool` (`KismetMathLibrary.And_IntInt` (`KismetMathLibrary.Conv_BoolToInt` (== (`self.CurrentSq`) _sq)) (`KismetMathLibrary.Conv_BoolToInt` (== _dialog (`self.CurrentDialogue`)))))
                    (`TextBlock.SetText` (`/Game/Blueprints/UI/WB_Dialogue.TB_Dialogue` (`self.DialogueWidget`)) (`KismetTextLibrary.Conv_StringToText` _dialoguetext))
                    (if (== _lastdialogue true)
                      (`self.EndDialogue`)
                      (return)
                      (else
                        (for _ _ :!via `Break`
                          _))))))))))
      (:`Is Not Valid`
        (return)))))

(fn `StartDialogue`
  (`|ExecutionSequence`
    (:`then_0`
      (bind _returnvalue (`|CreateWidget` "/Game/Blueprints/UI/WB_Dialogue.WB_Dialogue_C" (`GameplayStatics.GetPlayerController` 0)))
      (set `self.DialogueWidget` _returnvalue)
      (bind _output_get (set `/Game/Blueprints/UI/WB_Dialogue.NPC_Ref` self (`self.DialogueWidget`)))
      (`UserWidget.AddToViewport` (`/Game/Blueprints/BP_NPC_Base.DialogueWidget` _output_get) 0))
    (:`then_1`
      (set `self.CurrentSq` 1))
    (:`then_2`
      (set `self.CurrentDialogue` 0))
    (:`then_3`
      (`self.ShowNextDialogue`))
    (:`then_4`
      (`WidgetBlueprintLibrary.SetInputMode_UIOnlyEx` (`GameplayStatics.GetPlayerController` 0) (`self.DialogueWidget`)))))

(fn `UserConstructionScript`)